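; Actor Blueprint that shows one of two static meshes depending on a sanity value.
; At BeginPlay it compares GetSanity against SanityThreshold once, using HighSanityMesh at or above the threshold and LowSanityMesh below it.
; The construction script picks between the same meshes from the HighSanity boolean, independent of the sanity value, so either state can appear in the editor.
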(event `self.ReceiveBeginPlay`
  (bind _staticmesh (`self.StaticMesh`))
  (bind _sanity (`/Game/StoryAdvTemplate/Blueprints/Sanity.GetSanity`))
  (if (>= _sanity (`self.SanityThreshold`))
    (`StaticMeshComponent.SetStaticMesh` _staticmesh (`self.HighSanityMesh`))
    (else
      (`StaticMeshComponent.SetStaticMesh` _staticmesh (`self.LowSanityMesh`)))))

(fn `UserConstructionScript`
  (bind _staticmesh (`self.StaticMesh`))
  (if (`self.HighSanity?`)
    (`StaticMeshComponent.SetStaticMesh` _staticmesh (`self.HighSanityMesh`))
    (else
      (`StaticMeshComponent.SetStaticMesh` _staticmesh (`self.LowSanityMesh`)))))