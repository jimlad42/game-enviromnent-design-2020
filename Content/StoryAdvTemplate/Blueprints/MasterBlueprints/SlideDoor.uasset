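; SlideDoor is a sliding door Blueprint that toggles between two positions each time its Interaction event fires.
; An Open flag selects whether Timeline_0 plays forward or reverses, and flips on each interaction.
; The timeline's track drives a vector lerp between DoorStart and DoorEnd, setting the door object's relative location without sweep.
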(event `self.Interaction`
  (if (`self.Open`)
    (set `self.Open` false)
    (bind (_direction _newtrack_0) (`Timeline|Timeline_0` :!label _label)
      (:`Update`
        (`SceneComponent.K2_SetRelativeLocation` (`self.Object`) (`KismetMathLibrary.VLerp` (`self.DoorStart`) (`self.DoorEnd`) _newtrack_0) false false)))
    (else
      (set `self.Open` true)
      (goto _label :!via `Reverse`))))

(fn `UserConstructionScript`
  (`parent.UserConstructionScript`))