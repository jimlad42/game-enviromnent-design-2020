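; Sanity helper functions that read and modify the player's Sanity value on BP_FirstPersonCharacter.
; GetSanity and ChangeSanity cast player character 0 to that class, then return its Sanity or forward a shift to its ChangeSanity.
; SetSanity imitates an absolute set by applying a fixed -100 shift followed by SanityShift, leaving its Sanity input unused.
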(fn `ChangeSanity`
  (params (SanityShift :type "Float (double-precision)"))
  ;[1 1 1] Change Sanity
  (bind _asbp_first_person_character (cast `/Game/StoryAdvTemplate/Blueprints/BP_FirstPersonCharacter` (`GameplayStatics.GetPlayerCharacter` null)))
  (`/Game/StoryAdvTemplate/Blueprints/BP_FirstPersonCharacter.Change Sanity` _asbp_first_person_character SanityShift))

(fn `GetSanity`
  (returns (Sanity :type "Float (double-precision)"))
  (bind _asbp_first_person_character (cast `/Game/StoryAdvTemplate/Blueprints/BP_FirstPersonCharacter` (`GameplayStatics.GetPlayerCharacter` null)))
  (return (`/Game/StoryAdvTemplate/Blueprints/BP_FirstPersonCharacter.Sanity` _asbp_first_person_character)))

(fn `SetSanity`
  (params (Sanity :type "Float (double-precision)") (SanityShift :type "Float (double-precision)"))
  (`self.ChangeSanity` -100.0)
  (`self.ChangeSanity` SanityShift))