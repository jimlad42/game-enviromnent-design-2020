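; SlideDoor is a sliding door that responds to interaction only when the game controller holds its matching key ID.
; It caches the first BP_GameController at BeginPlay, then checks that controller's KeyIDs on each Interaction.
; A successful check plays the door audio and toggles the Open flag, playing or reversing a timeline.
; The timeline lerps the door object's relative location between DoorStart and DoorEnd.
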(event `self.ReceiveBeginPlay`
  (bind _outactors (`GameplayStatics.GetAllActorsOfClass` "/Game/Blueprints/MainBlueprints/BP_GameController.BP_GameController_C"))
  (set `self.GameControllerInstance` (`|GetArrayItem` _outactors))
  (`AudioComponent.Stop` (`self.Audio`)))

(event `self.Interaction`
  (if (`KismetArrayLibrary.Array_Contains` (`/Game/Blueprints/MainBlueprints/BP_GameController.KeyIDs` (`self.GameControllerInstance`)) (`self.KeyID`))
    (`AudioComponent.Play` (`self.Audio`) 1.0)
    (if (`self.Open`)
      (set `self.Open` false)
      (bind (_direction _newtrack_0) (`Timeline|Timeline_0` :!label _label)
        (:`Update`
          (`SceneComponent.K2_SetRelativeLocation` (`self.Object`) (`KismetMathLibrary.VLerp` (`self.DoorStart`) (`self.DoorEnd`) _newtrack_0) false false)))
      (else
        (set `self.Open` true)
        (goto _label :!via `Reverse`)))))

(fn `UserConstructionScript`
  (`parent.UserConstructionScript`))