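; AI controller for the Monster that runs its behavior tree and feeds it the player character and patrol target locations through the blackboard.
; It gathers all PatrolPath actors at start and steps through the current path's points.
; When a path runs out, it picks a different random path and teleports the monster to its first point.
; The perception update handler queries perceived actors but does nothing with the results.
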(event `self.ReceiveBeginPlay`
  (`self.RunBehaviorTree` "/Game/Blueprints/Monster/Monster_BT.Monster_BT")
  (bind _asmonster (cast `/Game/Blueprints/Monster/Monster` (`self.K2_GetPawn`)))
  (set `self.MonsterInstance` _asmonster)
  (`BlackboardComponent.SetValueAsObject` (`AIBlueprintHelperLibrary.GetBlackboard` null) "Player Character" (`GameplayStatics.GetPlayerCharacter` 0))
  (bind _outactors (`GameplayStatics.GetAllActorsOfClass` "/Game/Blueprints/Monster/OtherBlueprints/PatrolPath.PatrolPath_C"))
  (bind _output_get (set `self.PatrolPaths` _outactors))
  (set `self.CurrentPatrol` (`|GetArrayItem` _output_get))
  (`self.GetNextPatrolPoint`))

(event `self.AIPerception.OnPerceptionUpdated`
  (params (UpdatedActors :type "Array of Actor Object Reference (by ref)"))
  (for _array_element UpdatedActors
    (`AIPerceptionComponent.GetActorsPerception` (`self.AIPerception`) _array_element)))

(fn `ChoosePatrol`
  (locals (TestingPatrol :type "/Game/Blueprints/Monster/OtherBlueprints/PatrolPath Object Reference"))
  (bind _output_get (set `local.TestingPatrol` (`self.GetRandomPatrol`) :!label _label))
  (if (== (`self.CurrentPatrol`) _output_get)
    (goto _label)
    (else
      (set `self.CurrentPatrol` _output_get)
      (set `self.PatrolPoint` 0))))

(fn `GetNextPatrolPoint`
  (bind _currentpatrol (`self.CurrentPatrol`))
  (bind _currentpatrol_2 (`self.CurrentPatrol`))
  (if (not (`KismetArrayLibrary.Array_IsValidIndex` (`/Game/Blueprints/Monster/OtherBlueprints/PatrolPath.PatrolPoints` (`self.CurrentPatrol`)) (`self.PatrolPoint`)))
    (`self.ChoosePatrol`)
    (`self.K2_TeleportTo` :`self` (`self.K2_GetPawn`) :`DestLocation` (+ (+ (`self.K2_GetActorLocation` _currentpatrol_2) (`|GetArrayItem` (`/Game/Blueprints/Monster/OtherBlueprints/PatrolPath.PatrolPoints` _currentpatrol_2) (`self.PatrolPoint`))) (0.0 0.0 100.0))))
  (`BlackboardComponent.SetValueAsVector` (`AIBlueprintHelperLibrary.GetBlackboard` null) "TargetLocation" (+ (`self.K2_GetActorLocation` _currentpatrol) (`|GetArrayItem` (`/Game/Blueprints/Monster/OtherBlueprints/PatrolPath.PatrolPoints` _currentpatrol) (`self.PatrolPoint`))))
  (`/Engine/EditorBlueprintResources/StandardMacros.IncrementInt` (`self.PatrolPoint`)))

(fn `UserConstructionScript`)