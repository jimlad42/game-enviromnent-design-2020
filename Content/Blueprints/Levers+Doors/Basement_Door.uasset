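; Basement door Blueprint that unlocks progress once enough linked levers are active.
; Activated raises or lowers an active lever count and prints it to screen.
; When the count reaches LeversRequired, it sets a one-shot HasActivated flag and calls ChangeSanity with a fixed amount.
; The construction script only runs the parent's logic; no door movement happens in these graphs.
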(fn `Activated`
  (params (`Active?` :type Boolean))
  (bind _activatelevers (`self.ActivateLevers`))
  (if `Active?`
    (bind _result (`/Engine/EditorBlueprintResources/StandardMacros.IncrementInt` _activatelevers)
      (:`  `
        (`KismetSystemLibrary.PrintString` (`KismetStringLibrary.Conv_IntToString` _result))))
    (else
      (bind _result_2 (`/Engine/EditorBlueprintResources/StandardMacros.DecrementInt` _activatelevers)
        (:`  `
          (`KismetSystemLibrary.PrintString` (`KismetStringLibrary.Conv_IntToString` _result_2))))))
  (if (and (>= (`self.ActivateLevers`) (`self.LeversRequired`)) (not (`self.Has Activated`)))
    (set `self.Has Activated` true)
    (`/Game/Blueprints/MainBlueprints/Sanity.ChangeSanity` 100.0)))

(fn `UserConstructionScript`
  (`parent.UserConstructionScript`))