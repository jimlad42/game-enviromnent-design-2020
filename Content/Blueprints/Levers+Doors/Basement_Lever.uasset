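; Basement lever interactable that switches a linked InteractedItem on and off and resets itself after a hold time.
; Each Interaction alternates a FlipFlop, passes the Active state to InteractedItem, and plays or reverses a timeline that pitches the lever mesh.
; When the forward swing finishes, a HeldTime timer re-fires Interaction to flip it back; finishing the backward swing clears that timer.
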(event `self.Interaction`
  (bind _staticmesh (`self.StaticMesh`))
  (bind _interacted_item (`self.Interacted Item`))
  (bind _isa (`/Engine/EditorBlueprintResources/StandardMacros.FlipFlop`)
    (:`A`
      (bind _output_get (set `self.Active?` _isa))
      (`/Game/Blueprints/Levers+Doors/Activated_Object_Master.Activated` _interacted_item _output_get)
      (bind (_direction _newtrack_1) (`Timeline|Timeline_0` :!label _label)
        (:`Update`
          (`SceneComponent.K2_SetRelativeRotation` _staticmesh (`KismetMathLibrary.MakeRotator` (.roll (`SceneComponent.RelativeRotation` _staticmesh)) _newtrack_1 (.yaw (`SceneComponent.RelativeRotation` _staticmesh))) false false))
        (:`Finished`
          (switch `ETimelineDirection` _direction
            (:`Forward`
              (bind _returnvalue (`KismetSystemLibrary.K2_SetTimerDelegate` (delegate `self.Interaction`) (`self.Held_Time`))))
            (:`Backward`
              (`KismetSystemLibrary.K2_ClearAndInvalidateTimerHandle` _returnvalue))))))
    (:`B`
      (bind _output_get_2 (set `self.Active?` _isa))
      (`/Game/Blueprints/Levers+Doors/Activated_Object_Master.Activated` _interacted_item _output_get_2)
      (goto _label :!via `Reverse`))))

(fn `UserConstructionScript`
  (`parent.UserConstructionScript`))