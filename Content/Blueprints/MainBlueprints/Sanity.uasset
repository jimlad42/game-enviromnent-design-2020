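; Sanity is a set of helper functions for reading and modifying the player's sanity level.
; Each function casts player character 0 to BP_FirstPersonCharacter, then reads its Sanity variable or forwards to its SetSanity or ChangeSanity function.
; The sanity value lives on the character, so these functions only act as a shortcut to it and do nothing further if the cast fails.
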(fn `ChangeSanity`
  (params (SanityShift :type "Float (double-precision)"))
  ;[1 1 1] Change Sanity
  (bind _asbp_first_person_character (cast `/Game/Blueprints/MainBlueprints/BP_FirstPersonCharacter` (`GameplayStatics.GetPlayerCharacter` null)))
  (`/Game/Blueprints/MainBlueprints/BP_FirstPersonCharacter.Change Sanity` _asbp_first_person_character SanityShift))

(fn `GetSanity`
  (returns (Sanity :type "Float (double-precision)"))
  (bind _asbp_first_person_character (cast `/Game/Blueprints/MainBlueprints/BP_FirstPersonCharacter` (`GameplayStatics.GetPlayerCharacter` null)))
  (return (`/Game/Blueprints/MainBlueprints/BP_FirstPersonCharacter.Sanity` _asbp_first_person_character)))

(fn `SetSanity`
  (params (SanityLevel :type "Float (double-precision)"))
  (bind _asbp_first_person_character (cast `/Game/Blueprints/MainBlueprints/BP_FirstPersonCharacter` (`GameplayStatics.GetPlayerCharacter` null)))
  (`/Game/Blueprints/MainBlueprints/BP_FirstPersonCharacter.SetSanity` _asbp_first_person_character SanityLevel))